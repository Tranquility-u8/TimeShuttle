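; Anim notify placed in enemy death montages to mark the enemy as dead when the montage finishes.
; On trigger it casts the mesh owner to BP_Enemy and skips if the reverse montage component is reversing time.
; Otherwise it sets Dead in the enemy's Status struct and resets the custom montage with zero blend-out.
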(fn ReceivedNotify
  (params (MeshComp :type Skeletal%20Mesh%20Component%20Object%20Reference) (Animation :type Anim%20Sequence%20Base%20Object%20Reference))
  (bind _asbp_enemy (Utilities|Casting|CastToBP_Enemy (Components|GetOwner MeshComp))
    (:then
      (if (Default|IsReversingProperty (Variables|/Game/TimeReverseSystem/Blueprints/Enemy/BP_Enemy.BP_Enemy_C|GetBP_ReverseAnimMontageComponent _asbp_enemy))
        (return false)
        (else
          (Utilities|Struct|SetmembersinSCharacterStatus (Variables|/Game/TimeReverseSystem/Blueprints/Enemy/BP_Enemy.BP_Enemy_C|GetStatus _asbp_enemy) true)
          (Default|ResetCustomMontage _asbp_enemy 0.0)
          (return true))))
    (:CastFailed
      (return false))))

(fn GetNotifyName
  (return "FinishDeathMontage"))