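; Enemy character for a time-reversal system, with hit points, death and resurrection when time is rewound.
; Reverse component delegates toggle the AI blackboard's Reversing flag; finishing a rewind broadcasts resurrection if the Dead status is false.
; Tick updates a camera-facing HP widget and records speed in the Status struct except while reversing.
; Lethal damage disables capsule collision, broadcasts death and plays the death montage through helpers that track the current montage.
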(event Custom|Die
  (Collision|SetCollisionEnabled (Variables|Collision|GetCapsuleComponent) "NoCollision")
  (Default|CallOnDied)
  ;[1 1 1] Dead by montage notification
  (CallFunction|PlayCustomMontage "/Game/TimeReverseSystem/Characters/Animations/AM_Death.AM_Death" 1.0 0.0 "None"))

(event Custom|OnStartReversingActorTransform
  ;[1 1 1] When you start rewinding, set it on the blackboard
  (AI|Components|Blackboard|SetValueasBool (Variables|/Script/AIModule.AIController|GetBlackboard (Variables|Default|GetAIController)) (Utilities|Name|MakeLiteralName "Reversing") true))

(event Custom|OnFinishReversingActorTransform
  ;[1 1 1] When rewinding is finished, set the blackboard to finish rewinding
  (AI|Components|Blackboard|SetValueasBool (Variables|/Script/AIModule.AIController|GetBlackboard (Variables|Default|GetAIController)) (Utilities|Name|MakeLiteralName "Reversing") false)
  ;[1 1 1] Resuscitate if not dead
  (if (not (.Dead (Utilities|Struct|BreakSCharacterStatus (Variables|Default|GetStatus))))
    (Default|CallOnResurrected)))

(event Custom|PlayCustomMontage
  (params (MontageToPlay :type Anim%20Montage%20Object%20Reference) (PlayRate :type Float%20%28double-precision%29) (StartingPosition :type Float%20%28double-precision%29) (StartingSection :type Name))
  ;[1 1 1] Custom Anim Montage Event
  (bind _output_get (Variables|Default|SetCurrentMontage MontageToPlay))
  (Animation|Montage|PlayMontage (Variables|Character|GetMesh) _output_get PlayRate StartingPosition StartingSection
    (:OnCompleted
      (Variables|Default|SetCurrentMontage 0))))

(event Custom|ResetCustomMontage
  (params (InBlendOutTime :type Float%20%28double-precision%29) (Montage :type Anim%20Montage%20Object%20Reference))
  ;[1 1 1] Custom Anim Montage Reset
  (Variables|Default|SetCurrentMontage 0)
  (Animation|Montage|MontageStop (Components|SkeletalMesh|GetAnimInstance (Variables|Character|GetMesh)) InBlendOutTime Montage))

(event Game|Damage|EventAnyDamage
  (params (Damage :type Float%20%28single-precision%29) (DamageType :type Damage%20Type%20Object%20Reference) (InstigatedBy :type Controller%20Object%20Reference) (DamageCauser :type Actor%20Object%20Reference))
  (bind _status (Variables|Default|GetStatus))
  (bind _hitpoint (Utilities|Struct|BreakSCharacterStatus _status))
  (bind _returnvalue (- _hitpoint Damage))
  ;[1 1 1] If enemy hit point drops below 0, enemy will die.
  (if (not (Utilities|Struct|BreakSCharacterStatus (Variables|Default|GetStatus)))
    (if (<= _returnvalue 0.0)
      ;[1 1 1] Die Enemy
      (if (!= (Utilities|Struct|BreakSCharacterStatus (Variables|Default|GetStatus)) 0.0)
        (Utilities|Struct|SetmembersinSCharacterStatus (Variables|Default|GetStatus) 0.0)
        (CallFunction|Die))
      (else
        (Utilities|Struct|SetmembersinSCharacterStatus (Variables|Default|GetStatus) _returnvalue)))))

(event EventBeginPlay
  ;[1 1 1] When you start rewinding, set it on the blackboard
  (EventDispatchers|AssignOnStartReversingActorProperty (Variables|Default|GetBP_ReverseTrasnsformComponent) (delegate Custom|OnStartReversingActorTransform))
  ;[1 1 1] When rewinding is finished, set the blackboard to finish rewinding
  (EventDispatchers|AssignOnFinishReversingActorProperty (Variables|Default|GetBP_ReverseTrasnsformComponent) (delegate Custom|OnFinishReversingActorTransform)))

(event EventTick
  (params (DeltaSeconds :type Float%20%28single-precision%29))
  (UserInterface|SetEnemyHitPointGauge)
  (if (not (Default|IsReversingProperty (Variables|Default|GetBP_ReverseStatusComponent)))
    (Utilities|Struct|SetmembersinSCharacterStatus (Variables|Default|GetStatus) (Math|Vector|VectorLength (Transformation|GetVelocity)))))

(fn ConstructionScript)

(fn SetEnemyHitPointGauge
  (Transformation|SetWorldRotation (Variables|Default|GetHPWidget) (Math|Rotator|FindLookatRotation (Transformation|GetWorldLocation (Variables|Default|GetHPWidget)) (Camera|GetCameraLocation (Game|GetPlayerCameraManager 0))) false false)
  (bind _aswbp_enemy_hp (Utilities|Casting|CastToWBP_EnemyHP (UserInterface|GetUserWidgetObject (Variables|Default|GetHPWidget))))
  (Rendering|Components|TextRender|SetText (Variables|/Game/TimeReverseSystem/Widgets/WBP_EnemyHP.WBP_EnemyHP_C|GetCurrentHPText _aswbp_enemy_hp) (Utilities|Text|ToText(Float) (.HitPoint (Utilities|Struct|BreakSCharacterStatus (Variables|Default|GetStatus))) "HalfToEven"))
  (return))