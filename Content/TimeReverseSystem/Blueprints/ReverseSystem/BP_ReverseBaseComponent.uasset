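; Base component for a time-reverse system, letting an owner actor record its properties and play them back in reverse.
; On BeginPlay it registers with BP_ReverseSystemManager, retrying while none is found, and unregisters when the owner is destroyed.
; Looping timers drive recording and two reverse modes, auto and seek, with root physics simulation suspended while reversing.
; Record, reverse and can-reverse logic are empty stubs for child components to override.
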(event Custom|DeactivateAutoReverseMode
  ;[1 1 1] Auto Reverse Mode Switcher.
  (CallFunction|FinishAutoReversingActorProperty)
  ;;[1 1 1] Control the simulate physics to use the reverse system.
  (if (Variables|Record|GetOriginalOwnerSimulatePhysics)
    (bind _asprimitive_component (Utilities|Casting|CastToPrimitiveComponent (Variables|/Script/Engine.Actor|GetRootComponent (Components|GetOwner))))
    (Physics|SetSimulatePhysics _asprimitive_component true))
  (CallFunction|StartRecordingActorProperty))

(event Custom|ActivateAutoReverseMode
  ;[1 1 1] Auto Reverse Mode Switcher.
  (CallFunction|FinishRecordingActorProperty)
  ;;[1 1 1] Control the simulate physics to use the reverse system.
  (if (Variables|Record|GetOriginalOwnerSimulatePhysics)
    (bind _asprimitive_component (Utilities|Casting|CastToPrimitiveComponent (Variables|/Script/Engine.Actor|GetRootComponent (Components|GetOwner))))
    (Physics|SetSimulatePhysics _asprimitive_component false))
  (CallFunction|StartAutoReversingActorProperty))

(event Custom|DeactivateSeekReverseMode
  ;[1 1 1] Seek Reverse Mode Switcher.
  (CallFunction|FinishSeekReversingActorProperty)
  ;;[1 1 1] Control the simulate physics to use the reverse system.
  (if (Variables|Record|GetOriginalOwnerSimulatePhysics)
    (bind _asprimitive_component (Utilities|Casting|CastToPrimitiveComponent (Variables|/Script/Engine.Actor|GetRootComponent (Components|GetOwner))))
    (Physics|SetSimulatePhysics _asprimitive_component true))
  (CallFunction|StartRecordingActorProperty))

(event Custom|ActivateSeekReverseMode
  ;[1 1 1] Seek Reverse Mode Switcher.
  (CallFunction|FinishRecordingActorProperty)
  ;;[1 1 1] Control the simulate physics to use the reverse system.
  (if (Variables|Record|GetOriginalOwnerSimulatePhysics)
    (bind _asprimitive_component (Utilities|Casting|CastToPrimitiveComponent (Variables|/Script/Engine.Actor|GetRootComponent (Components|GetOwner))))
    (Physics|SetSimulatePhysics _asprimitive_component false))
  (CallFunction|StartSeekReversingActorProperty))

(event Custom|FinishAutoReversingActorProperty
  ;[1 1 1] Auto Reverse Property.
  (Utilities|Time|ClearandInvalidateTimerbyHandle (Variables|Reverse|GetReversingTimer))
  (Default|CallOnFinishReversingActorProperty))

(event Custom|StartAutoReversingActorProperty
  ;[1 1 1] Auto Reverse Property.
  (bind _returnvalue (Utilities|Time|SetTimerbyEvent (EventDispatchers|CreateEvent :!event Custom|CheckIfActorCanReverseProperty) (CallFunction|GetRecordInterval) true))
  (Variables|Reverse|SetReversingTimer _returnvalue)
  (Default|CallOnStartReversingActorProperty))

(event Custom|ControlSeekReversingActorProperty
  (params (SeekBaseValue :type Float%20%28single-precision%29))
  ;[1 1 1] Seek Reverse property.
  ;;[1 1 1] Calculate Seek axis.
  (Variables|Reverse|Seek|SetSeekAxis (+ (Variables|Reverse|Seek|GetSeekAxis) (* (Math|Float|Truncate (Math|Float|Clamp(Float) SeekBaseValue -1.0)) (Math|Float|Truncate (/ (CallFunction|GetSeekReverseSecond) (CallFunction|GetRecordInterval)))))))

(event Custom|ReverseActorProperty
  ;[1 1 1] Auto Reverse Property.
  ;;[1 0 0] Override
)

(event Custom|CheckIfActorCanReverseProperty
  ;[1 1 1] Auto Reverse Property.
  (bind _reversesystemmanager (Variables|Reverse|GetReverseSystemManager)
    (:then
      (if (and (Reverse|CanReverseProperty) (>= (Default|GetCountdownTimerElapsedTime _reversesystemmanager) 0.1))
        (CallFunction|ReverseActorProperty)
        (else
          (Utilities|Time|ClearandInvalidateTimerbyHandle (Variables|Reverse|GetReversingTimer))
          (Default|CallOnbeLimitOfReverse))))
    (:else)))

(event Custom|SeekReverseActorProperty
  ;[1 1 1] Seek Reverse property.
)

(event Custom|RecordActorProperty
  ;[1 1 1] Record owner actor property.
  ;;[1 0 0] Override
)

(event Custom|StartRecordingActorProperty
  ;[1 1 1] Record owner actor property.
  (bind _returnvalue (Utilities|Time|SetTimerbyEvent (EventDispatchers|CreateEvent :!event Custom|RecordActorProperty) (CallFunction|GetRecordInterval) true))
  (Variables|Record|SetRecordingTimer _returnvalue)
  (Default|CallOnStartRecordingActorProperty))

(event Custom|OnDestroyedOwnerActor
  (params (DestroyedActor :type Actor%20Object%20Reference))
  ;[1 1 1] Cancel registration from "Reverse System Manager" when owner actor destroyed.
  (Default|RemoveItemfromReversibleComponents (Variables|Reverse|GetReverseSystemManager) self))

(event Custom|FinishRecordingActorProperty
  ;[1 1 1] Record owner actor property.
  (Utilities|Time|ClearandInvalidateTimerbyHandle (Variables|Record|GetRecordingTimer))
  (Default|CallOnFinishRecordingActorProperty))

(event Custom|SetUpReverseSystem
  ;[1 1 1] Get Reverse System Manager. (Time out after 5 counts)
  (Utilities|FlowControl|DoN 5
    (:Exit
      (bind _outactors (Actor|GetAllActorsOfClass "/Game/TimeReverseSystem/Blueprints/ReverseSystem/Controller/BP_ReverseSystemManager.BP_ReverseSystemManager_C"))
      (if (Utilities|Array|IsValidIndex _outactors)
        (Variables|Reverse|SetReverseSystemManager (Utilities|Array|Get(acopy) _outactors))
        ;[1 1 1] Register for "Reverse System Manager".
        (Default|AddUniqueItemforReversibleComponents (Variables|Reverse|GetReverseSystemManager) self)
        (Utilities|FlowControl|Sequence
          (:then_0
            (CallFunction|StartRecordingActorProperty)
            ;[1 1 1] Get owner's simulate physics state.
            (bind _asprimitive_component (Utilities|Casting|CastToPrimitiveComponent (Variables|/Script/Engine.Actor|GetRootComponent (Components|GetOwner))))
            (if (Class|SceneComponent|IsAnySimulatingPhysics _asprimitive_component)
              (Variables|Record|SetOriginalOwnerSimulatePhysics true)
              (else
                (Variables|Record|SetOriginalOwnerSimulatePhysics false))))
          (:then_1
            ;[1 1 1] Cancel registration from "Reverse System Manager" when owner actor destroyed.
            (Game|AssignOnDestroyed (Components|GetOwner) (delegate Custom|OnDestroyedOwnerActor))))
        (else
          (Utilities|FlowControl|Delay 0.2)
          (CallFunction|SetUpReverseSystem))))))

(event Custom|FinishSeekReversingActorProperty
  ;[1 1 1] Seek Reverse property.
  (Utilities|Time|ClearandInvalidateTimerbyHandle (Variables|Reverse|GetReversingTimer))
  (Default|CallOnFinishReversingActorProperty))

(event Custom|StartSeekReversingActorProperty
  ;[1 1 1] Seek Reverse property.
  (bind _returnvalue (Utilities|Time|SetTimerbyEvent (EventDispatchers|CreateEvent :!event Custom|SeekReverseActorProperty) (CallFunction|GetRecordInterval) true))
  (Variables|Reverse|SetReversingTimer _returnvalue)
  (Default|CallOnStartReversingActorProperty))

(event EventBeginPlay
  ;[1 0 0] Important process.
  (CallFunction|SetUpReverseSystem))

(fn IsRecordingProperty
  (return (Class|KismetSystemLibrary|TimerExistsHandle (Variables|Record|GetRecordingTimer))))

(fn IsReversingProperty
  (return (Class|KismetSystemLibrary|TimerExistsHandle (Variables|Reverse|GetReversingTimer))))

(fn CanReverseProperty
  (return false))

(fn GetAnimationPlayRate
  (return (Variables|Reverse|GetAnimationPlayRate)))