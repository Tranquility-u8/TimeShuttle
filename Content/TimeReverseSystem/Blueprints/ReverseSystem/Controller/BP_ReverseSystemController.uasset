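; BP_ReverseSystemController is the control layer for the time-reverse system, exposing auto reverse, seek reverse and tutorial-window toggling.
; On BeginPlay it finds BP_ReverseSystemManager in the level, retrying briefly a limited number of times, and creates the HUD widget.
; Its events check the manager's current mode to keep auto and seek exclusive, then drive the manager, HUD and reverse-time post-process.
; Seek mode toggles through a FlipFlop and forwards a value for scrubbing.
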(event Custom|SetUpReverseSystem
  ;[1 0 0] Set up for use Reverse System.
  ;;[1 1 1] Get Reverse System Manager. (Time out after 5 counts)
  (Utilities|FlowControl|DoN 5
    (:Exit
      (bind _outactors (Actor|GetAllActorsOfClass "/Game/TimeReverseSystem/Blueprints/ReverseSystem/Controller/BP_ReverseSystemManager.BP_ReverseSystemManager_C"))
      (if (Utilities|Array|IsValidIndex _outactors)
        (Variables|Default|SetReverseSystemManager (Utilities|Array|Get(acopy) _outactors))
        (else
          (Utilities|FlowControl|Delay 0.2)
          (CallFunction|SetUpReverseSystem))))))

(event Custom|ToggleTutorialWindow
  ;[1 1 1] Toggle Tutorial Window visivility.
  (bind _reversesystemhud (Variables|Default|GetReverseSystemHUD)
    (:then
      (Default|ToggleTutorialWindowAnimation _reversesystemhud))
    (:else)))

(event Custom|ActivateAutoReverseSystem
  ;[1 1 1] Control Auto Reverse System.
  (Utilities|IsReverseModeSameasComparison "NewEnumerator1"
    (:false
      (Default|ActivateAutoReverseMode (Variables|Default|GetReverseSystemManager))
      (bind _reversesystemhud (Variables|Default|GetReverseSystemHUD)
        (:then
          (Default|ActivateAutoReverseHUD _reversesystemhud))
        (:else
          _))
      (Default|PlayReverseTimePostProcess (Variables|Default|GetReverseSystemManager)))))

(event Custom|DeactivateAutoReverseSystem
  ;[1 1 1] Control Auto Reverse System.
  (Utilities|IsReverseModeSameasComparison "NewEnumerator0"
    (:true
      (Default|DeactivateAutoReverseMode (Variables|Default|GetReverseSystemManager))
      (bind _reversesystemhud (Variables|Default|GetReverseSystemHUD)
        (:then
          (Default|DeactivateAutoReverseHUD _reversesystemhud))
        (:else
          _))
      (Default|ReversePlayReverseTimePostProcess (Variables|Default|GetReverseSystemManager)))))

(event Custom|ToggleSeekReverseSystemMode
  ;[1 1 1] Control Seek Reverse System.
  (Utilities|IsReverseModeSameasComparison "NewEnumerator0"
    (:false
      (Utilities|FlowControl|FlipFlop
        (:A
          (Default|ActivateSeekReverseMode (Variables|Default|GetReverseSystemManager))
          (bind _reversesystemhud (Variables|Default|GetReverseSystemHUD)
            (:then
              (Default|ActivateSeekReverseHUD _reversesystemhud))
            (:else
              _))
          (Default|PlayReverseTimePostProcess (Variables|Default|GetReverseSystemManager)))
        (:B
          (Utilities|IsReverseModeSameasComparison "NewEnumerator1"
            (:true
              (Default|DeactivateSeekReverseMode (Variables|Default|GetReverseSystemManager))
              (bind _reversesystemhud_2 (Variables|Default|GetReverseSystemHUD)
                (:then
                  (Default|DeactivateSeekReverseHUD _reversesystemhud_2))
                (:else
                  _))
              (Default|ReversePlayReverseTimePostProcess (Variables|Default|GetReverseSystemManager)))))))))

(event Custom|ControlSeekReverseSystem
  (params (Value :type Float%20%28single-precision%29))
  ;[1 1 1] Control Seek Reverse System.
  (Utilities|IsReverseModeSameasComparison "NewEnumerator1"
    (:true
      (Default|ControlSeekReverse (Variables|Default|GetReverseSystemManager) Value))))

(event EventBeginPlay
  (CallFunction|SetUpReverseSystem)
  ;[1 1 1] Show Reverse System HUD.
  (bind _returnvalue (UserInterface|CreateWidget "/Game/TimeReverseSystem/Widgets/WBP_ReverseSystemHUD.WBP_ReverseSystemHUD_C"))
  (Utilities|IsValid _returnvalue
    (:Is%20Valid
      (bind _output_get (Variables|Default|SetReverseSystemHUD _returnvalue))
      (UserInterface|Viewport|AddtoViewport _output_get 0))))

(fn IsReversing
  (return (Utilities|Enum|NotEqual(Enum) (Default|GetReverseMode (Variables|Default|GetReverseSystemManager)) "NewEnumerator2")))