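; Time reversal manager that switches registered reversible components between normal, auto-reverse and seek-reverse modes.
; Mode changes broadcast to the components and restart a looping timer that maintains an elapsed-time clock, counting up normally and down during auto reverse.
; Seek axis input drives both components and clock, with rewinding clamped between the mode-entry time and the maximum recording window.
; A timeline fades post-process saturation and black clip for the reverse effect.
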(event Custom|StopCountdownTimer
  ;[1 1 1] Stop coundown timer.
  (Utilities|Time|ClearandInvalidateTimerbyHandle (Variables|CountdownTimer|GetCountdownTimer)))

(event Custom|ReversePlayReverseTimePostProcess
  ;[1 1 1] Change Post Process Settings for Reverse System.
  (bind _alpha (Timeline|ReverseTimePostProcessTimeline Reverse)
    (:Update
      (Utilities|Struct|SetmembersinPostProcessSettings (Variables|/Script/Engine.PostProcessComponent|GetSettings (Variables|Default|GetPostProcess)) (Math|Vector4|MakeVector4 (Math|Float|Lerp 1.0 0.0 _alpha) (Math|Float|Lerp 1.0 0.0 _alpha) (Math|Float|Lerp 1.0 0.0 _alpha) (Math|Float|Lerp 1.0 0.0 _alpha)) (Math|Float|Lerp 0.0 1.0 _alpha)))))

(event Custom|CalculateSeekReverseCountdownTimer
  (params (Value :type Float%20%28single-precision%29))
  ;[1 1 1] Calculate Timer to use Seek Reverse System.
  (Variables|CountdownTimer|SetElapsedTime (Math|Float|Clamp(Float) (+ Value (Variables|CountdownTimer|GetElapsedTime)) (select (<= (- (Variables|CountdownTimer|GetTemporaryElapsedTime) (CallFunction|GetMaxRecordingingSecond)) 0.0) 0.0 (- (Variables|CountdownTimer|GetTemporaryElapsedTime) (CallFunction|GetMaxRecordingingSecond))) (Variables|CountdownTimer|GetTemporaryElapsedTime))))

(event Custom|PlayReverseTimePostProcess
  ;[1 1 1] Change Post Process Settings for Reverse System.
  (bind _alpha (Timeline|ReverseTimePostProcessTimeline Play)
    (:Update
      (Utilities|Struct|SetmembersinPostProcessSettings (Variables|/Script/Engine.PostProcessComponent|GetSettings (Variables|Default|GetPostProcess)) (Math|Vector4|MakeVector4 (Math|Float|Lerp 1.0 0.0 _alpha) (Math|Float|Lerp 1.0 0.0 _alpha) (Math|Float|Lerp 1.0 0.0 _alpha) (Math|Float|Lerp 1.0 0.0 _alpha)) (Math|Float|Lerp 0.0 1.0 _alpha)))))

(event Custom|ControlSeekReverse
  (params (AxisValue :type Float%20%28single-precision%29))
  ;[1 1 1] Seek Reverse Mode
  (Default|ControlSeekReversingActorProperty (Variables|ReverseSystem|GetReversiblesComponents) AxisValue)
  (CallFunction|CalculateSeekReverseCountdownTimer (* (Math|Float|Clamp(Float) AxisValue -1.0) (CallFunction|GetSeekReverseSecond))))

(event Custom|DeactivateSeekReverseMode
  ;[1 1 1] Seek Reverse Mode
  (Default|DeactivateSeekReverseMode (Variables|ReverseSystem|GetReversiblesComponents))
  (bind _output_get (Variables|ReverseSystem|SetReverseMode "NewEnumerator2"))
  (CallFunction|SetUpCountdownTimer _output_get))

(event Custom|SetUpCountdownTimer
  (params (ReverseMode :type EReverseMode%20Enum :default "NewEnumerator0"))
  ;[1 1 1] Countdown Timer switcher
  (if (Utilities|Time|IsTimerActivebyHandle (Variables|CountdownTimer|GetCountdownTimer))
    (CallFunction|StopCountdownTimer))
  (bind _returnvalue (Utilities|Time|SetTimerbyEvent (Utilities|Select :Index ReverseMode :NewEnumerator0 (EventDispatchers|CreateEvent :!event Custom|CalculateAutoReverseCountdownTimer) :NewEnumerator1 (EventDispatchers|CreateEvent :!event Custom|StopCountdownTimer) :NewEnumerator2 (EventDispatchers|CreateEvent :!event Custom|CalculateNormalCountdownTimer)) (Variables|CountdownTimer|GetCountTime) true))
  (Variables|CountdownTimer|SetCountdownTimer _returnvalue)
  (Variables|CountdownTimer|SetTemporaryElapsedTime (Variables|CountdownTimer|GetElapsedTime)))

(event Custom|CalculateNormalCountdownTimer
  ;[1 1 1] Normal countdown timer calculation process.
  (Variables|CountdownTimer|SetElapsedTime (+ (Variables|CountdownTimer|GetElapsedTime) (Variables|CountdownTimer|GetCountTime))))

(event Custom|ActivateSeekReverseMode
  ;[1 1 1] Seek Reverse Mode
  (Default|ActivateSeekReverseMode (Variables|ReverseSystem|GetReversiblesComponents))
  (bind _output_get (Variables|ReverseSystem|SetReverseMode "NewEnumerator1"))
  (CallFunction|SetUpCountdownTimer _output_get))

(event Custom|ActivateAutoReverseMode
  ;[1 1 1] Auto Reverse Mode
  (Default|ActivateAutoReverseMode (Variables|ReverseSystem|GetReversiblesComponents))
  (bind _output_get (Variables|ReverseSystem|SetReverseMode "NewEnumerator0"))
  (CallFunction|SetUpCountdownTimer _output_get))

(event Custom|CalculateAutoReverseCountdownTimer
  ;[1 1 1] Countdown timer calculation process in reverse mode.
  (Variables|CountdownTimer|SetElapsedTime (Math|Float|Clamp(Float) (+ (Variables|CountdownTimer|GetElapsedTime) (* -1 (Variables|CountdownTimer|GetCountTime))) (select (<= (- (Variables|CountdownTimer|GetTemporaryElapsedTime) (CallFunction|GetMaxRecordingingSecond)) 0.0) 0.0 (- (Variables|CountdownTimer|GetTemporaryElapsedTime) (CallFunction|GetMaxRecordingingSecond))) (Variables|CountdownTimer|GetTemporaryElapsedTime))))

(event Custom|DeactivateAutoReverseMode
  ;[1 1 1] Auto Reverse Mode
  (Default|DeactivateAutoReverseMode (Variables|ReverseSystem|GetReversiblesComponents))
  (bind _output_get (Variables|ReverseSystem|SetReverseMode "NewEnumerator2"))
  (CallFunction|SetUpCountdownTimer _output_get))

(event EventBeginPlay
  ;[1 1 1] Set up countdown timer when started game.
  (bind _output_get (Variables|ReverseSystem|SetReverseMode "NewEnumerator2"))
  (CallFunction|SetUpCountdownTimer _output_get))

(fn ConstructionScript)

(fn GetCountdownTimerElapsedTime
  (return (Variables|CountdownTimer|GetElapsedTime)))

(fn GetReverseMode
  (return (Variables|ReverseSystem|GetReverseMode)))

(fn AddUniqueItemforReversibleComponents
  (params (NewItem :type BP%20Reverse%20Base%20Component%20Object%20Reference%20%28by%20ref%29))
  (bind _returnvalue (Utilities|Array|AddUnique (Variables|ReverseSystem|GetReversiblesComponents) NewItem))
  (return _returnvalue))

(fn RemoveItemfromReversibleComponents
  (params (RemoveItem :type BP%20Reverse%20Base%20Component%20Object%20Reference%20%28by%20ref%29))
  (bind _returnvalue (Utilities|Array|RemoveItem (Variables|ReverseSystem|GetReversiblesComponents) RemoveItem))
  (return _returnvalue))

(fn GetCountdownTimerTemporaryElapsedTime
  (return (Variables|CountdownTimer|GetTemporaryElapsedTime)))