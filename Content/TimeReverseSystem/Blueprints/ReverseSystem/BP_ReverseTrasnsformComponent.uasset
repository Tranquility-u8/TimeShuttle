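; Actor component in the time-reverse system that records its owner's transform and plays it back backwards.
; Recording keeps a rolling buffer sized by max seconds over interval; auto reverse pops the newest transform onto the owner.
; Seeking steps a temporary index through the buffer by seek axis, then trims later entries on release.
; It also sets an animation play rate to match playback direction, zero when seek is idle.
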(event EventCheckifActorCanReverseProperty
  ;[1 1 1] Auto Reverse Property.
  (|CallParentFunction))

(event EventStartSeekReversingActorProperty
  ;[1 1 1] Seek Reverse transform.
  (|CallParentFunction)
  (Variables|Default|SetTemporarySeekIndex (Utilities|Array|LastIndex (Variables|Default|GetRecordedTransforms))))

(event EventSeekReverseActorProperty
  ;[1 1 1] Seek Reverse transform.
  (|CallParentFunction)
  (Utilities|IsValid (Variables|Default|GetReverseSystemManager)
    (:Is%20Valid
      ;;[1 1 1] Is Seek Axis is Plus? Minus?
      (if (!= (Variables|Default|GetSeekAxis) 0)
        (if (> (Variables|Default|GetSeekAxis) 0)
          ;;[1 1 1] Seek play
          (if (<= (+ (Variables|Default|GetTemporarySeekIndex) 1) (Utilities|Array|LastIndex (Variables|Default|GetRecordedTransforms)))
            (Math|Integer|IncrementInt (Variables|Default|GetTemporarySeekIndex)
              (:%20%20
                (Transformation|SetActorTransform (Components|GetOwner) (Utilities|Array|Get(acopy) (Variables|Default|GetRecordedTransforms) (Variables|Default|GetTemporarySeekIndex)))
                (Math|Integer|DecrementInt (Variables|Default|GetSeekAxis)
                  (:%20%20
                    (Variables|Default|SetAnimationPlayRate 1.0)))))
            (else
              (Variables|Default|SetSeekAxis 0)))
          (else
            ;;[1 1 1] Seek Reverse
            (if (>= (- (Variables|Default|GetTemporarySeekIndex) 1) (Variables|Default|GetFirstSeekIndex))
              (Math|Integer|DecrementInt (Variables|Default|GetTemporarySeekIndex)
                (:%20%20
                  (Transformation|SetActorTransform (Components|GetOwner) (Utilities|Array|Get(acopy) (Variables|Default|GetRecordedTransforms) (Variables|Default|GetTemporarySeekIndex)))
                  (Math|Integer|IncrementInt (Variables|Default|GetSeekAxis)
                    (:%20%20
                      (Variables|Default|SetAnimationPlayRate -1.0)))))
              (else
                (Variables|Default|SetSeekAxis 0)))))
        (else
          (Variables|Default|SetAnimationPlayRate 0.0))))))

(event EventFinishSeekReversingActorProperty
  ;[1 1 1] Seek Reverse transform.
  (|CallParentFunction)
  (if (!= (Variables|Default|GetTemporarySeekIndex) (Utilities|Array|LastIndex (Variables|Default|GetRecordedTransforms)))
    ;;[1 1 1] Remove Index after unseek index when released seek.
    (bind _arrayindex (Utilities|Array|ReverseforEachLoop (Variables|Default|GetRecordedTransforms))
      (:LoopBody
        (if (>= _arrayindex (Variables|Default|GetTemporarySeekIndex))
          (Utilities|Array|RemoveIndex (Variables|Default|GetRecordedTransforms) _arrayindex)))
      (:Completed
        (Variables|Default|SetAnimationPlayRate 1.0 :!label _label)
        (Default|CallOnFinishReversingActorProperty)))
    (else
      (goto _label))))

(event EventControlSeekReversingActorProperty
  (params (SeekBaseValue :type Float%20%28single-precision%29))
  ;[1 1 1] Seek Reverse transform.
  (|CallParentFunction SeekBaseValue))

(event EventBeginPlay
  (|CallParentFunction))

(event EventRecordActorProperty
  ;[1 1 1] Record owner actor transform.
  (|CallParentFunction)
  (if (< (Utilities|Array|Length (Variables|Default|GetRecordedTransforms)) (Math|Float|Truncate (/ (CallFunction|GetMaxRecordingingSecond) (CallFunction|GetRecordInterval))))
    (Utilities|Array|Add (Variables|Default|GetRecordedTransforms) (Transformation|GetActorTransform (Components|GetOwner)))
    (else
      ;;[1 1 1] If you reach the recording limit when adding a new element, remove the beginning of the array and add.
      (Utilities|Array|RemoveIndex (Variables|Default|GetRecordedTransforms))
      (Utilities|Array|Add (Variables|Default|GetRecordedTransforms) (Transformation|GetActorTransform (Components|GetOwner))))))

(event EventStartRecordingActorProperty
  ;[1 1 1] Record owner actor transform.
  (|CallParentFunction))

(event EventFinishRecordingActorProperty
  ;[1 1 1] Record owner actor transform.
  (|CallParentFunction))

(event EventReverseActorProperty
  ;[1 1 1] Auto Reverse Property.
  (|CallParentFunction)
  ;;[1 1 1] Reverse owner actor transform.
  (Transformation|SetActorTransform (Components|GetOwner) (Utilities|Array|Get(acopy) (Variables|Default|GetRecordedTransforms) (Utilities|Array|LastIndex (Variables|Default|GetRecordedTransforms))))
  (Utilities|Array|RemoveIndex (Variables|Default|GetRecordedTransforms) (Utilities|Array|LastIndex (Variables|Default|GetRecordedTransforms))))

(event EventStartAutoReversingActorProperty
  ;[1 1 1] Auto Reverse Property.
  (|CallParentFunction)
  (Variables|Default|SetAnimationPlayRate -1.0))

(event EventFinishAutoReversingActorProperty
  ;[1 1 1] Auto Reverse Property.
  (|CallParentFunction)
  (Variables|Default|SetAnimationPlayRate 1.0))

(fn CanReverseProperty
  (return (> (Utilities|Array|LastIndex (Variables|Default|GetRecordedTransforms)) 0)))